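; BP_Ball_DM is a destructible ball actor that breaks apart when the third-person character collides with it.
; On a component hit from ThirdPersonCharacter it enables physics on the destructible mesh and applies small radial damage at the impact point, credited to the character's spear.
; One second later it destroys itself.
; A disconnected leftover would move the actor toward another object's ball component at constant speed.
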(event `self.Destructible.OnComponentHit`
  (params (HitComponent :type "PrimitiveComponent Object Reference") (OtherActor :type "Actor Object Reference") (OtherComp :type "PrimitiveComponent Object Reference") (NormalImpulse :type "Vector Structure") (Hit :type "HitResult Structure (by ref)"))
  (bind _asthird_person_character (cast `/Game/ThirdPersonBP/Blueprints/ThirdPersonCharacter` OtherActor))
  (`PrimitiveComponent.SetSimulatePhysics` (`self.Destructible`) true)
  (`GameplayStatics.ApplyRadialDamage` :`BaseDamage` 10.0 :`Origin` (`.ImpactPoint` (`GameplayStatics.BreakHitResult` Hit)) :`DamageRadius` 10.0 :`DamageCauser` (`/Game/ThirdPersonBP/Blueprints/ThirdPersonCharacter.spearRef` _asthird_person_character) :`InstigatedByController` null)
  (`KismetSystemLibrary.Delay` 1.0)
  (`self.K2_DestroyActor`))

(fn `UserConstructionScript`)